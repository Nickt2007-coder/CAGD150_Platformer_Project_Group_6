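; BP_Enemy1 is a side-scroller patrol enemy that the player defeats by jumping on it.
; Tick feeds a WhereToGo vector into movement input at reduced scale, and each Hit event flip-flops that vector between the two X directions.
; When BP_SideScrollerCharacter overlaps HeadCollider, the enemy removes the collider, stops moving, squashes and lowers its capsule, then destroys itself after a short delay.
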(event `self.ReceiveTick`
  (params (DeltaSeconds :type "Float (single-precision)"))
  ; Move Enemy Every Frame based on Vector
  (`self.AddMovementInput` (`self.WhereToGo`) 0.5))

(event `self.ReceiveHit`
  (params (MyComp :type "PrimitiveComponent Object Reference") (Other :type "Actor Object Reference") (OtherComp :type "PrimitiveComponent Object Reference") (bSelfMoved :type Boolean) (HitLocation :type "Vector Structure") (HitNormal :type "Vector Structure") (NormalImpulse :type "Vector Structure") (Hit :type "HitResult Structure (by ref)"))
  ; Switch Movement Diection on Hit
  (`/Engine/EditorBlueprintResources/StandardMacros.FlipFlop`
    (:`A`
      (set `self.WhereToGo` (-1.0 0.0 0.0)))
    (:`B`
      (set `self.WhereToGo` (1.0 0.0 0.0)))))

(event `self.Head Collider.OnComponentBeginOverlap`
  (params (OverlappedComponent :type "PrimitiveComponent Object Reference") (OtherActor :type "Actor Object Reference") (OtherComp :type "PrimitiveComponent Object Reference") (OtherBodyIndex :type Integer) (bFromSweep :type Boolean) (SweepResult :type "HitResult Structure (by ref)"))
  (bind _capsulecomponent (`self.CapsuleComponent`))
  ; Die When Jumped On
  (cast `/Game/Johnny-Work/Blueprints/BP_SideScrollerCharacter` OtherActor)
  (`ActorComponent.K2_DestroyComponent` (`self.Head Collider`))
  (`MovementComponent.StopMovementImmediately` (`self.CharacterMovement`))
  (`CharacterMovementComponent.DisableMovement` (`self.CharacterMovement`))
  (`SceneComponent.SetWorldScale3D` _capsulecomponent (1.0 1.0 0.5))
  (`KismetSystemLibrary.MoveComponentTo` _capsulecomponent (- (`SceneComponent.RelativeLocation` _capsulecomponent) (0.0 0.0 20.0)) (struct) false false 0.1)
  (`KismetSystemLibrary.Delay` 0.2)
  (`self.K2_DestroyActor`))

(fn `UserConstructionScript`)