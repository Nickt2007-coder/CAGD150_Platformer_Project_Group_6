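; BP_BaseBrick is a side-scroller brick that switches to a broken look when overlapped while the player is jumping.
; On overlap it reads the jump flag from player 0's BP_SideScrollerCharacter, without checking the overlapping actor or hit direction, and swaps the Cube's material.
; IsBroken is set before the jump check, so a first overlap without jumping also uses up the one-time change.
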(event `self.ReceiveActorBeginOverlap`
  (params (OtherActor :type "Actor Object Reference"))
  ;[0 0.03128 0.15 0.5] ChangeBrick Texture when hit from bottom
  (bind _asbp_side_scroller_character (cast `/Game/Johnny-Work/Blueprints/BP_SideScrollerCharacter` (`GameplayStatics.GetPlayerPawn` 0)))
  (if (not (`self.IsBroken`))
    (set `self.IsBroken` true)
    (if (`/Game/Johnny-Work/Blueprints/BP_SideScrollerCharacter.Is Jumpoing` _asbp_side_scroller_character)
      (`PrimitiveComponent.SetMaterial` (`self.Cube`) 0 "/Game/Christian-work/Christian-Materials/M_BrickBroken.M_BrickBroken")
      (cast `/Game/Johnny-Work/Blueprints/BP_SideScrollerCharacter` (`GameplayStatics.GetPlayerPawn` 0)))))

(fn `UserConstructionScript`)