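; BP_Enemy_3 is a side-scroller enemy Blueprint that pauses after touching the player character.
; On a hit with BP_SideScrollerCharacter, it zeroes WhereToGo and disables its collision.
; After a five-second delay, it restores collision and sets WhereToGo to negative X, whatever its earlier heading.
; Construction and StompReaction only call the parent class, and its own Tick is disabled.
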(event `self.ReceiveHit`
  (params (MyComp :type "PrimitiveComponent Object Reference") (Other :type "Actor Object Reference") (OtherComp :type "PrimitiveComponent Object Reference") (bSelfMoved :type Boolean) (HitLocation :type "Vector Structure") (HitNormal :type "Vector Structure") (NormalImpulse :type "Vector Structure") (Hit :type "HitResult Structure (by ref)"))
  (cast `/Game/Johnny-Work/Blueprints/BP_SideScrollerCharacter` Other)
  (set `self.Where To Go` (0.0 0.0 0.0))
  (`self.SetActorEnableCollision` false)
  (`KismetSystemLibrary.Delay` 5.0)
  (`self.SetActorEnableCollision` true)
  (set `self.Where To Go` (-1.0 0.0 0.0)))

(fn `StompReaction`
  (`parent.StompReaction`))

(fn `UserConstructionScript`
  (`parent.UserConstructionScript`))