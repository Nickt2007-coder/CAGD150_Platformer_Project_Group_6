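; BP_CheckPoint is a spinning, single-use checkpoint pickup for the side-scroller character.
; On overlap with BP_SideScrollerCharacter, it stores its location and sets a checkpoint flag in BP_GameInstance.
; It then destroys itself, plays a flagpole sound and prints a checkpoint message.
; Tick applies a fixed local rotation every frame without delta-time scaling, alongside a zero world offset that moves nothing.
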(event `self.ReceiveActorBeginOverlap`
  (params (OtherActor :type "Actor Object Reference"))
  (cast `/Game/Johnny-Work/Blueprints/BP_SideScrollerCharacter` OtherActor)
  (bind _asbp_game_instance (cast `/Game/Christian-work/BP_GameInstance` (`GameplayStatics.GetGameInstance`)))
  (set `/Game/Christian-work/BP_GameInstance.CheckPoint` (`self.K2_GetActorLocation`) _asbp_game_instance)
  (set `/Game/Christian-work/BP_GameInstance.HasCheckPoint` true _asbp_game_instance)
  (`self.K2_DestroyActor`)
  (`GameplayStatics.PlaySound2D` "/Game/Johnny-Work/Audio/super-mario-down-the-flag-pole-sound-effect.super-mario-down-the-flag-pole-sound-effect" 1.0 1.0 0.0 null null)
  (`KismetSystemLibrary.PrintString` "Checkpoint!!" true true (struct :`R` 1.0 :`G` 0.293666 :`B` 0.967642 :`A` 1.0)))

(event `self.ReceiveTick`
  (params (DeltaSeconds :type "Float (single-precision)"))
  (`self.K2_AddActorLocalRotation` (struct :`Yaw` 60.0))
  (`self.K2_AddActorWorldOffset` (0.0 0.0 0.0)))

(fn `UserConstructionScript`)