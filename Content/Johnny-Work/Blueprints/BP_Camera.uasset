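; BP_Camera is an actor that follows the side-scroller player character at a configurable offset.
; BeginPlay caches the player character, and Tick moves the actor to that character's location plus Offset, with sweep enabled.
; The construction script applies the same offset, without sweep, to the BP_SideScrollerCharacter found in the level, so the actor is already positioned before play begins.
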(event `self.ReceiveBeginPlay`
  ; Store ref to player
  (bind _asbp_side_scroller_character (cast `/Game/Johnny-Work/Blueprints/BP_SideScrollerCharacter` (`GameplayStatics.GetPlayerCharacter` 0)))
  (set `self.PlayerRef` _asbp_side_scroller_character))

(event `self.ReceiveTick`
  (params (DeltaSeconds :type "Float (single-precision)"))
  ;[0.15 0.03304 0.03232 0.5] Set camera position to player's position + offset
  (`self.K2_SetActorLocation` (+ (`self.K2_GetActorLocation` (`self.PlayerRef`)) (`self.Offset`)) true))

(fn `UserConstructionScript`
  (bind _returnvalue (`GameplayStatics.GetActorOfClass` "/Game/Johnny-Work/Blueprints/BP_SideScrollerCharacter.BP_SideScrollerCharacter_C"))
  (`self.K2_SetActorLocation` (+ (`self.K2_GetActorLocation` _returnvalue) (`self.Offset`))))